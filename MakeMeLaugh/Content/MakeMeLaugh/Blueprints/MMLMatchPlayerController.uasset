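; Match player controller that spawns and possesses either the monster or player pawn for its player.
; On BeginPlay, the local controller reads IsMonster from MMLGameInstance and passes the matching pawn class to ServerSpawnPawn.
; That event spawns the pawn at InitialTransform, which SetInitialTransform stores through ServerSetInitialTransform, and then possesses it.
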(event Custom|Server%20Spawn%20Pawn
  (params (Pawn%20Class :type Pawn%20Class%20Reference))
  ;[1 1 1] Server Spawn Pawn
  (bind _returnvalue (Game|SpawnActorfromClass Pawn%20Class (Variables|Default|GetInitial%20Transform) "Undefined" 0 0))
  (Pawn|Possess _returnvalue))

(event Custom|Set%20Initial%20Transform
  (params (Transform :type Transform))
  ;[1 1 1] Set Initial Transform
  (CallFunction|ServerSetInitialTransform Transform))

(event Custom|Server%20Set%20Initial%20Transform
  (params (Transform :type Transform))
  ;[1 1 1] Set Initial Transform
  (Variables|Default|SetInitial%20Transform Transform))

(event EventBeginPlay
  ;[1 1 1] Begin Play
  (if (Pawn|IsLocalPlayerController)
    (bind _asmmlgame_instance (Utilities|Casting|CastToMMLGameInstance (Game|GetGameInstance)))
    (CallFunction|ServerSpawnPawn (select (Variables|/Game/MakeMeLaugh/Blueprints/MMLGameInstance.MMLGameInstance_C|GetIs%20Monster _asmmlgame_instance) "/Game/MakeMeLaugh/Blueprints/Monster/MonsterBlueprint.MonsterBlueprint_C" "/Game/MakeMeLaugh/Blueprints/Player/PlayerBlueprint.PlayerBlueprint_C"))))

(fn ConstructionScript)