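; Lobby game mode that tracks connected players and starts the match.
; Player logins are stored in a list and notify the first top-level lobby menu widget, and logouts remove the controller from it.
; Starting the match picks a random player controller to be the monster, then runs a server travel to the gameplay map.
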(event Custom|Start%20Match
  (Default|SetasMonster (.AsMMLLobby%20Player%20Controller (Utilities|Casting|CastToMMLLobbyPlayerController (.OutItem (Utilities|Array|Random (Variables|Default|GetPlayers))))))
  (Development|ExecuteConsoleCommand "servertravel ThirdPersonExampleMap" 0))

(event EventPostLogin
  (params (NewPlayer :type Player%20Controller%20Object%20Reference))
  (Utilities|Array|Add (Variables|Default|GetPlayers) NewPlayer)
  (bind _foundwidgets (Widget|GetAllWidgetsOfClass "/Game/MakeMeLaugh/Blueprints/UI/LobbyMenuWidget.LobbyMenuWidget_C" true))
  (Default|PlayerLogin (Utilities|Array|Get(acopy) _foundwidgets)))

(event EventOnLogout
  (params (ExitingController :type Controller%20Object%20Reference))
  (bind _asplayer_controller (Utilities|Casting|CastToPlayerController ExitingController))
  (Utilities|Array|RemoveItem (Variables|Default|GetPlayers) _asplayer_controller))

(fn ConstructionScript)